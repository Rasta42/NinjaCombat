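; Gameplay Ability for the player's melee combo attack, playing ComboMontages in sequence at increased speed.
; A Player.Action.Attack gameplay event received during a montage queues the next one on completion; otherwise, or after the last montage, the ability ends.
; The "Damage" montage notify runs a sphere overlap in front of the owner, applying point damage and spawning a hit particle for each actor found.
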(event `self.K2_ActivateAbility`
  (set `self.AttackIndex` 0)
  (`self.NextAttack`))

(event `NextAttack`
  (bind _attackindex (`self.AttackIndex`))
  (bind ((`OwnerActor` _owneractor) (`PlayerController` _playercontroller)) (break `GameplayAbilityActorInfo` (`self.GetActorInfo`)))
  (bind ((`OwnerActor` _owneractor_2)) (break `GameplayAbilityActorInfo` (`self.GetActorInfo`)))
  (bind _returnvalue (`Actor.GetActorForwardVector` _owneractor_2))
  (bind _returnvalue_2 (+ (`Actor.K2_GetActorLocation` _owneractor_2) (* _returnvalue 100.0)))
  (set `self.NeedNextAttack` false)
  (bind _notifyname (`|PlayMontage` (`.SkeletalMeshComponent` (break `GameplayAbilityActorInfo` (`self.GetActorInfo`))) (`|GetArrayItem` (`self.ComboMontages`) (`self.AttackIndex`)) 1.3)
    (:`then`
      (`AbilityTask_WaitGameplayEvent.WaitGameplayEvent` (struct :`TagName` "Player.Action.Attack") null true
        (:`EventReceived`
          (set `self.NeedNextAttack` true))))
    (:`OnCompleted`
      (if (and (`self.NeedNextAttack`) (> (`KismetArrayLibrary.Array_LastIndex` (`self.ComboMontages`)) _attackindex))
        (`/Engine/EditorBlueprintResources/StandardMacros.IncrementInt` _attackindex
          (:`  `
            (`self.NextAttack`)))
        (else
          (`self.K2_EndAbility`))))
    (:`OnNotifyBegin`
      (if (== _notifyname "Damage")
        (bind _outactors (`KismetSystemLibrary.SphereOverlapActors` _returnvalue_2 50.0 (`|MakeArray` "ObjectTypeQuery2" "ObjectTypeQuery3" :!type "EObjectTypeQuery Enum") null (`|MakeArray` _owneractor_2))) ; Simple check enemies front of player
        (for _array_element _outactors
          (`GameplayStatics.ApplyPointDamage` _array_element 100.0 _returnvalue (`GameplayStatics.MakeHitResult` true false 0.0 0.0 _returnvalue_2) _playercontroller _owneractor)
          (`GameplayStatics.SpawnEmitterAtLocation` "/Game/Particles/P_Hit.P_Hit" _returnvalue_2 (struct) (0.5 0.5 0.5)))))))