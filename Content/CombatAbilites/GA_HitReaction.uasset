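; Gameplay ability that plays escalating hit reaction montages on its owner and lets it smash props it collides with.
; Each Player.Hitted gameplay event advances an index into ComboMontages and plays the next reaction, ending when a montage completes or the list runs out.
; While active, it binds the owner's OnActorHit and destroys any BaseProp touched from the third reaction onward.
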(event `self.K2_ActivateAbility`
  (set `self.AttackIndex` 0)
  (`self.NextHit`)
  (add `Actor.OnActorHit` (`.OwnerActor` (break `GameplayAbilityActorInfo` (`self.GetActorInfo`))) (delegate `HitProp`)))

(event `HitProp`
  (params (SelfActor :type "Actor Object Reference") (OtherActor :type "Actor Object Reference") (NormalImpulse :type "Vector Structure") (Hit :type "HitResult Structure (by ref)"))
  (bind _asbase_prop (cast `/Game/Props/BaseProp` OtherActor))
  (if (>= (`self.AttackIndex`) 2)
    (`Actor.K2_DestroyActor` _asbase_prop)))

(event `self.K2_OnEndAbility`
  (params (bWasCancelled :type Boolean))
  (remove `Actor.OnActorHit` (`.OwnerActor` (break `GameplayAbilityActorInfo` (`self.GetActorInfo`))) (`|CreateDelegate` :!event `HitProp`)))

(event `NextHit`
  (set `self.NeedNextAttack` false)
  (if (`KismetArrayLibrary.Array_IsValidIndex` (`self.ComboMontages`) (`self.AttackIndex`))
    (`|PlayMontage` (`.SkeletalMeshComponent` (break `GameplayAbilityActorInfo` (`self.GetActorInfo`))) (`|GetArrayItem` (`self.ComboMontages`) (`self.AttackIndex`))
      (:`then`
        (`AbilityTask_WaitGameplayEvent.WaitGameplayEvent` (struct :`TagName` "Player.Hitted") null true
          (:`EventReceived`
            (`/Engine/EditorBlueprintResources/StandardMacros.IncrementInt` (`self.AttackIndex`)
              (:`  `
                (`self.NextHit`))))))
      (:`OnCompleted`
        (`self.K2_EndAbility` :!label _label)))
    (else
      (goto _label))))